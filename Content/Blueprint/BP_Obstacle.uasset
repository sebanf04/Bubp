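; Paper2D asteroid obstacle that kills the player by opening level L_Nivel1 when BP_Charater overlaps it.
; BeginPlay picks one of three flipbooks at random for its sprite.
; Tick compares its height to a threshold re-rolled every frame; once reached, it rotates the sprite and enables physics and gravity on Sphere1.
; The actor destroys itself after a short delay.
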(event EventBeginPlay
  (Sprite|SetFlipbook (Variables|Default|Getasteroid) (Utilities|Array|Get(acopy) (Variables|Default|GetFlipbook) (Math|Random|RandomIntegerinRange 0 2))))

(event EventTick
  (params (DeltaSeconds :type Float%20%28single-precision%29))
  (bind _sphere1 (Variables|Default|GetSphere1))
  (Utilities|FlowControl|Sequence
    (:then_0
      (if (<= (Math|Random|RandomFloatinRange 9e+02 1.3e+03) (.z (Transformation|GetActorLocation)))
        (Transformation|SetRelativeRotation (Variables|Default|Getasteroid) "0.000000,-90.000000,-180.000000" false false)
        (Physics|SetSimulatePhysics _sphere1 true)
        (Physics|SetEnableGravity _sphere1 true)
        (Utilities|FlowControl|Delay 3.5)
        (Actor|DestroyActor)))))

(event Collision|EventActorBeginOverlap
  (params (OtherActor :type Actor%20Object%20Reference))
  ;[1 1 1] MATA AL PERSONAJE
  (Utilities|Casting|CastToBP_Charater OtherActor)
  (Game|OpenLevel(byName) "L_Nivel1"))

(fn ConstructionScript)